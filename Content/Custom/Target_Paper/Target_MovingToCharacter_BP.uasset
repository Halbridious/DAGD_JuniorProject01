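; A VR shooting target pawn that chases the player and ends the game if it reaches them.
; Tick reissues an AI move toward the player, with the cube's look-at rotation applied when the move completes.
; WasHit notifies the Accuracy actor and, unless Dead, plays a sound, updates the Score actor and teleports to a random navigable point around TargetOrigin.
; Sphere overlap with the MotionControllerPawn quits after a short delay.
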(event OnComponentBeginOverlap(Sphere)
  (params (OverlappedComponent :type Primitive%20Component%20Object%20Reference) (OtherActor :type Actor%20Object%20Reference) (OtherComp :type Primitive%20Component%20Object%20Reference) (OtherBodyIndex :type Integer) (bFromSweep :type Boolean) (SweepResult :type Hit%20Result%20Structure%20%28by%20ref%29))
  ;[1 1 1] enemy reaches player
  (Utilities|Casting|CastToMotionControllerPawn OtherActor)
  (Development|PrintString "game over")
  (Utilities|FlowControl|Delay 1.0)
  (Game|QuitGame 0 "Quit"))

(event EventTick
  (params (DeltaSeconds :type Float%20%28single-precision%29))
  ;[1 1 1] look at player
  (AI|AIMoveTo self "0, 0, 0" (Game|Player|GetPlayerPawn 0) 5.0 false
    (:then
      (Transformation|SetWorldRotation (Variables|Default|GetCube) (Math|Rotator|FindLookatRotation (Transformation|GetWorldLocation (Variables|Default|GetCube)) (Transformation|GetActorLocation (Game|Player|GetPlayerPawn 0))) false false))))

(event EventWasHit
  ;[1 1 1] Target was hit
  (bind _outactors (Actor|GetAllActorsOfClass "/Game/Custom/Functionality/Score.Score_C"))
  (Variables|Default|SetScoreBoard (Utilities|Array|Get(acopy) _outactors))
  (bind _outactors_2 (Actor|GetAllActorsOfClass "/Game/Custom/Guns/glock/Accuracy.Accuracy_C"))
  (Default|Score (Utilities|Array|Get(acopy) _outactors_2))
  (if (not (Variables|Default|GetDead))
    (Audio|PlaySound2D "/Game/Custom/Sounds/Audio/Collapse01.Collapse01")
    (Class|ScoreInterface|Score(Message) (Variables|Default|GetScoreBoard))
    (Transformation|Teleport (.RandomLocation (Class|NavigationSystem|GetRandomPointinNavigableRadius (Variables|Default|GetTargetOrigin) 5e+03)) "0, 0, 0")))

(event EventBeginPlay
  (Audio|PlaySoundatLocation "/Game/Custom/Sounds/Audio/Starter_Music_Cue.Starter_Music_Cue" (Transformation|GetActorLocation)))

(fn ConstructionScript)