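; Timer actor that counts down and restarts play by opening the Homecoming_IntroDemo level when time runs out.
; Tick runs a one-second Delay, then decrements the Timer variable and writes it to a TextRender component.
; Because Delay ignores retriggers while pending, the per-frame Tick yields roughly one decrement per second.
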(event EventTick
  (params (DeltaSeconds :type Float%20%28single-precision%29))
  ;[0.0446 1 0] Timer
  (Utilities|FlowControl|Delay 1.0)
  (bind _output_get (Variables|Default|SetTimer (- (Variables|Default|GetTimer) 1)))
  (Rendering|Components|TextRender|SetText (Variables|Default|GetTextRender) (Utilities|Text|ToText(Integer) _output_get))
  (if (<= (Variables|Default|GetTimer) 0)
    (Game|OpenLevel(byName) "Homecoming_IntroDemo")))

(fn ConstructionScript)