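; Accuracy display Blueprint that shows the player's shooting accuracy as a percentage on a TextRender component.
; WasHit and BulletsFired events increment float counters for targets hit and shots fired.
; Tick divides hits by shots every frame, truncates the percentage to an integer and writes it to the text, with no explicit check for zero shots.
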(event EventWasHit
  ;[0.0446 1 0] Accuracy
  (bind _output_get (Variables|Default|SetTargetsHit (+ (Variables|Default|GetTargetsHit) 1.0))))

(event EventBulletsFired
  ;[0.0446 1 0] Accuracy
  (bind _output_get (Variables|Default|SetBulletsFired (+ (Variables|Default|GetBulletsFired) 1.0))))

(event EventTick
  (params (DeltaSeconds :type Float%20%28single-precision%29))
  ;[0.0446 1 0] Accuracy
  (Rendering|Components|TextRender|SetText (Variables|Default|GetTextRender) (Utilities|Text|ToText(Integer) (Math|Float|Truncate (* (/ (stale EventWasHit _output_get) (stale EventBulletsFired _output_get)) 1e+02)))))

(fn ConstructionScript)