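; Semi-automatic Glock pistol actor that can be picked up, dropped and fired.
; Interact alternates between attaching the gun to the given hand and detaching it, adjusting its offset and collision and toggling the crosshair.
; While held, Action spawns a bullet at the Shoot point with a sound.
; Short delays sequence the recoil, faked by nudging the slide mesh back and forward, around a casing spawned at the Ejection point.
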(event EventAction
  (bind _shoot (Variables|Default|GetShoot))
  (bind _returnvalue (Transformation|GetWorldTransform _shoot))
  ;[1 1 1] Fire Bullet
  (if (Variables|Default|GetHolding)
    (Game|SpawnActorfromClass "/Game/Custom/Bullet1.Bullet1_C" (Math|Transform|MakeTransform (.location _returnvalue) (.rotation _returnvalue) "1,1,1") "Undefined" 0 0)
    (Audio|PlaySoundatLocation "/Game/Custom/Sounds/Audio/Explosion01.Explosion01" (Transformation|GetActorLocation) "0, 0, 0" 0.25)
    (CallFunction|GunFunction01)
    (Utilities|FlowControl|Delay 0.01)
    (CallFunction|BulletEjection)
    (Utilities|FlowControl|Delay 0.01)
    (CallFunction|GunFunction02)))

(event EventInteract
  (params (Hand :type Scene%20Component%20Object%20Reference))
  (bind _glockbottom (Variables|Default|GetGlockBottom))
  (bind _defaultsceneroot (Variables|Default|GetDefaultSceneRoot))
  (Utilities|FlowControl|FlipFlop
    (:A
      ;[1 1 1] Pick up
      (Transformation|AttachComponentToComponent Hand "None" "SnapToTarget" "SnapToTarget" "KeepWorld" true)
      (Collision|SetCollisionEnabled _glockbottom "NoCollision")
      (Transformation|AddLocalRotation _defaultsceneroot "-45.000000,0.000000,0.000000" false false) ; Fix rotation
      (Transformation|AddLocalOffset _glockbottom "2.000000, 0, 0" false false) ; Fix Location
      (Variables|Default|SetHolding true)
      (Rendering|ToggleVisibility (Variables|Default|GetCrossHairs) false))
    (:B
      ;[1 1 1] Drop
      (Transformation|DetachFromActor "KeepWorld" "KeepWorld" "KeepWorld")
      (Collision|SetCollisionEnabled _glockbottom "QueryAndPhysics")
      (Transformation|AddLocalRotation _defaultsceneroot "45.000000,0.000000,0.000000" false false) ; Fix rotation
      (Transformation|AddLocalOffset _glockbottom "-2.000000, 0, 0" false false) ; Fix Location
      (Variables|Default|SetHolding false)
      (Rendering|ToggleVisibility (Variables|Default|GetCrossHairs) false))))

(fn ConstructionScript
  (|CallParentFunction))

(fn GunFunction01
  (Transformation|AddLocalOffset (Variables|Default|GetGlockTop) "-1.000000, 0, 0" false false))

(fn GunFunction02
  (Transformation|AddLocalOffset (Variables|Default|GetGlockTop) "1.000000, 0, 0" false false))

(fn BulletEjection
  (Game|SpawnActorfromClass "/Game/VirtualRealityBP/Blueprints/BulletEject_BP.BulletEject_BP_C" (Math|Transform|MakeTransform (.location (Transformation|GetWorldTransform (Variables|Default|GetEjection))) "0, 0, 0" "1,1,1") "Undefined" 0 0))