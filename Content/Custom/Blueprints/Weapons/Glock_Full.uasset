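; Fully automatic Glock weapon that attaches to a hand and fires while held.
; Interact alternates pickup and drop through a FlipFlop, toggling mesh collision and correcting the grip transform.
; Action starts a looping FullAuto timer that the Drop event clears.
; Each shot line-traces from Shoot, plays sound and impact effects, ejects a casing, reports to the Accuracy actor and notifies hit BPI_Enemy actors.
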(event Custom|FullAuto
  (bind _shoot (Variables|Default|GetShoot))
  (bind _returnvalue (Transformation|GetWorldTransform _shoot))
  ;[1 1 1] Fire Bullet
  (if (Variables|Default|GetHolding)
    (bind _outhit (Collision|LineTraceByChannel (.location _returnvalue) (+ (.location _returnvalue) (* (Math|Vector|GetForwardVector (.rotation _returnvalue)) 5e+03)) "TraceTypeQuery1" true 0 "None"))
    (Variables|Default|SetHitActor (.HitActor (Collision|BreakHitResult _outhit)))
    (Audio|PlaySoundatLocation "/Game/Custom/Sounds/GunShot.GunShot" (Transformation|GetActorLocation) "0, 0, 0" 0.25)
    (CallFunction|BulletEjection)
    (bind _outactors (Actor|GetAllActorsOfClass "/Game/Custom/Blueprints/Accuracy.Accuracy_C"))
    (Class|ScoreInterface|BulletsFired(Message) (Utilities|Array|Get(acopy) _outactors))
    (Effects|SpawnEmitteratLocation "/Game/Custom/Particles/Particles/BulletSplash.BulletSplash" (.Location (Collision|BreakHitResult _outhit)))
    (if (Utilities|DoesObjectImplementInterface (Variables|Default|GetHitActor) "/Game/VirtualRealityBP/Blueprints/BPI_Enemy.BPI_Enemy_C")
      (Class|BPIEnemy|WasHit(Message) (Variables|Default|GetHitActor)))))

(event EventDrop
  ;[1 1 1] Fire Bullet
  (Utilities|Time|ClearandInvalidateTimerbyHandle (stale EventAction _returnvalue)))

(event EventAction
  ;[1 1 1] Fire Bullet
  (if (Variables|Default|GetHolding)
    (bind _returnvalue (Utilities|Time|SetTimerbyEvent (delegate Custom|FullAuto) 0.1 true))))

(event EventInteract
  (params (Hand :type Scene%20Component%20Object%20Reference))
  (bind _defaultsceneroot (Variables|Default|GetDefaultSceneRoot))
  (bind _skeletalmesh (Variables|Default|GetSkeletalMesh))
  (bind _sphere (Variables|Default|GetSphere))
  (Utilities|FlowControl|FlipFlop
    (:A
      ;[1 1 1] Pick up
      (Transformation|AttachComponentToComponent Hand "None" "SnapToTarget" "SnapToTarget" "KeepWorld" true)
      (Collision|SetCollisionEnabled _skeletalmesh "NoCollision")
      (Transformation|AddLocalRotation _defaultsceneroot "-45.000000,0.000000,0.000000" false false) ; Fix rotation
      (Transformation|AddLocalOffset _skeletalmesh "2.000000, 0, 0" false false) ; Fix Location
      (Rendering|ToggleVisibility _sphere false)
      (Variables|Default|SetHolding true))
    (:B
      ;[1 1 1] Drop
      (Transformation|DetachFromActor "KeepWorld" "KeepWorld" "KeepWorld")
      (Collision|SetCollisionEnabled _skeletalmesh "QueryAndPhysics")
      (Transformation|AddLocalRotation _defaultsceneroot "45.000000,0.000000,0.000000" false false) ; Fix rotation
      (Transformation|AddLocalOffset _skeletalmesh "-2.000000, 0, 0" false false) ; Fix Location
      (Rendering|ToggleVisibility _sphere false)
      (Variables|Default|SetHolding false))))

(fn ConstructionScript
  (|CallParentFunction))

(fn GunFunction01)

(fn GunFunction02)

(fn BulletEjection
  (Game|SpawnActorfromClass "/Game/VirtualRealityBP/Blueprints/BulletEject_BP.BulletEject_BP_C" (Math|Transform|MakeTransform (.location (Transformation|GetWorldTransform (Variables|Default|GetEjection))) "0, 0, 0" "1,1,1") "Undefined" 0 0))