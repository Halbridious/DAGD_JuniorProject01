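; Hand-held Glock pistol actor that can be picked up, dropped and fired, despite the MainMenu asset name.
; Interact flip-flops between snapping it to the given hand and detaching it, toggling GlockBottom collision and applying matching rotation and location corrections.
; Action fires only while held, spawning a Bullet at the Shoot component's transform and playing a gunshot sound.
; Physics simulation toggles are present but unconnected, so they never run.
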(event EventAction
  (bind _shoot (Variables|Default|GetShoot))
  (bind _returnvalue (Transformation|GetWorldTransform _shoot))
  ;[1 1 1] Fire Bullet
  (if (Variables|Default|GetHolding)
    (Game|SpawnActorfromClass "/Game/Custom/Bullet.Bullet_C" (Math|Transform|MakeTransform (.location _returnvalue) (.rotation _returnvalue) "1,1,1") "Undefined" 0 0)
    (Audio|PlaySoundatLocation "/Game/Custom/Sounds/GunShot.GunShot" (Transformation|GetActorLocation) "0, 0, 0" 0.25)))

(event EventInteract
  (params (Hand :type Scene%20Component%20Object%20Reference))
  (bind _glockbottom (Variables|Default|GetGlockBottom))
  (bind _defaultsceneroot (Variables|Default|GetDefaultSceneRoot))
  (Utilities|FlowControl|FlipFlop
    (:A
      ;[1 1 1] Pick up
      (Transformation|AttachComponentToComponent Hand "None" "SnapToTarget" "SnapToTarget" "KeepWorld" true)
      (Collision|SetCollisionEnabled _glockbottom "NoCollision")
      (Transformation|AddLocalRotation _defaultsceneroot "-45.000000,0.000000,0.000000" false false) ; Fix rotation
      (Transformation|AddLocalOffset _glockbottom "2.000000, 0, 0" false false) ; Fix Location
      (Variables|Default|SetHolding true))
    (:B
      ;[1 1 1] Drop
      (Transformation|DetachFromActor "KeepWorld" "KeepWorld" "KeepWorld")
      (Collision|SetCollisionEnabled _glockbottom "QueryAndPhysics")
      (Transformation|AddLocalRotation _defaultsceneroot "45.000000,0.000000,0.000000" false false) ; Fix rotation
      (Transformation|AddLocalOffset _glockbottom "-2.000000, 0, 0" false false) ; Fix Location
      (Variables|Default|SetHolding false))))

(fn ConstructionScript
  (|CallParentFunction))