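; Target pawn that wanders once to a random spot and can be shot down.
; On first tick it AI-moves to a random ground point, then destroys itself a second after the move succeeds or fails.
; Lethal damage or a 9mm bullet hit destroys it with a sound, while WasHit destroys it silently.
; Scoring is an empty stub, and the TargetPoint cached at construction is unused.
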(event OnComponentHit(Mesh)
  (params (HitComponent :type Primitive%20Component%20Object%20Reference) (OtherActor :type Actor%20Object%20Reference) (OtherComp :type Primitive%20Component%20Object%20Reference) (NormalImpulse :type Vector :default "0, 0, 0") (Hit :type Hit%20Result%20Structure%20%28by%20ref%29))
  ;[1 1 1] If hit kills actor
  (Utilities|Casting|CastTo9mm_Bullet OtherActor)
  (Actor|DestroyActor)
  (Audio|PlaySound2D 0)
  ;;[1 1 1] Add Score
  (Utilities|Casting|CastToMotionControllerPawn OtherActor))

(event EventWasHit
  (Actor|DestroyActor))

(event Game|Damage|EventAnyDamage
  (params (Damage :type Float%20%28single-precision%29) (DamageType :type Damage%20Type%20Object%20Reference) (InstigatedBy :type Controller%20Object%20Reference) (DamageCauser :type Actor%20Object%20Reference))
  ;[1 1 1] If hit kills actor
  (bind _output_get (Variables|Default|SetCurrentHealth (- (Variables|Default|GetCurrentHealth) Damage)))
  (if (<= _output_get 0.0)
    (Actor|DestroyActor)
    (Audio|PlaySound2D 0)
    ;;[1 1 1] Add Score
    (Utilities|Casting|CastToMotionControllerPawn (stale OnComponentHit(Mesh) OtherActor))))

(event EventTick
  (params (DeltaSeconds :type Float%20%28single-precision%29))
  ;[1 1 1] Changes target point
  (Utilities|FlowControl|DoOnce false
    (:Completed
      ;[1 1 1] Moves to target point
      (AI|AIMoveTo self (Math|Vector|MakeVector (Math|Random|RandomFloatinRange 0.0 1e+04) (Math|Random|RandomFloatinRange 0.0 1e+04) 0.0) 0 5.0 false
        (:OnSuccess
          _)
        (:OnFail
          _))
      (Utilities|FlowControl|Delay 1.0)
      (Actor|DestroyActor))))

(fn ConstructionScript
  (bind _outactors (Actor|GetAllActorsOfClass "/Script/Engine.TargetPoint"))
  (Variables|Default|SetPoint (Utilities|Array|Get(acopy) _outactors)))