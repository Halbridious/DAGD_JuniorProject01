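; Stationary target that falls over when hit, notifies the scoreboard and stands back up after a short delay.
; The WasHit event finds the first Score actor in the level and, if the target is not already down, plays a collapse sound and calls ScoreMessage on it.
; It tips the Arrow component a quarter turn, using a Dead flag to ignore further hits until the rotation is reversed.
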(event EventWasHit
  ;[1 1 1] Target was hit
  (bind _outactors (Actor|GetAllActorsOfClass "/Game/Custom/Blueprints/Score.Score_C"))
  (Variables|Default|SetScoreBoard (Utilities|Array|Get(acopy) _outactors))
  (if (not (Variables|Default|GetDead))
    (Audio|PlaySound2D "/Game/Custom/Sounds/Audio/Collapse01.Collapse01")
    (Class|ScoreInterface|Score(Message) (Variables|Default|GetScoreBoard))
    (Transformation|AddLocalRotation (Variables|Default|GetArrow) "0,-90.000000, 0" false false)
    (Variables|Default|SetDead true)
    (Utilities|FlowControl|Delay 5.0)
    (Transformation|AddLocalRotation (Variables|Default|GetArrow) "0,90.000000, 0" false false)
    (Variables|Default|SetDead false)))

(fn ConstructionScript)