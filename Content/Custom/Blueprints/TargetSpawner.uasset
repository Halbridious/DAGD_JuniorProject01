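; Target spawner that spawns AI enemy or friendly targets at its Arrow transform in timed rounds.
; Tick re-triggers chained Delays, so targets spawn every Timer seconds while NewRound is true, with a random roll favoring friendlies.
; After about 30 seconds spawning pauses briefly, then Timer shortens, the first Wave actor's ScoreMessage fires and the next, faster round begins.
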(event Custom|SpawnTarget
  (bind _arrow (Variables|Default|GetArrow))
  (bind _returnvalue (Transformation|GetWorldLocation _arrow))
  (bind _returnvalue_2 (Transformation|GetWorldRotation _arrow))
  ;[1 1 1] Spawns target every few seconds
  (if (<= (Math|Random|RandomFloatinRange -3.0 5.0) 0.0)
    (AI|SpawnAIFromClass "/Game/Custom/Blueprints/TargetEnemy_BP.TargetEnemy_BP_C" 0 _returnvalue _returnvalue_2 false)
    (else
      (AI|SpawnAIFromClass "/Game/Custom/Blueprints/TargetFriendly_BP.TargetFriendly_BP_C" 0 _returnvalue _returnvalue_2 false))))

(event EventTick
  (params (DeltaSeconds :type Float%20%28single-precision%29))
  (if (Variables|Default|GetNew%20Round)
    (Utilities|FlowControl|Delay (Variables|Default|GetTimer))
    (CallFunction|SpawnTarget)
    (Utilities|FlowControl|Delay 3e+01)
    (Variables|Default|SetNew%20Round false)
    (Utilities|FlowControl|Delay 1e+01)
    (Variables|Default|SetTimer (- (Variables|Default|GetTimer) 0.25))
    (bind _outactors (Actor|GetAllActorsOfClass "/Game/Custom/Blueprints/Wave.Wave_C"))
    (Class|ScoreInterface|Score(Message) (Utilities|Array|Get(acopy) _outactors))
    (Variables|Default|SetNew%20Round true)))

(fn ConstructionScript)