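; Moving score target that slides back and forth and can be knocked down when hit.
; Tick nudges the Arrow component along local Z each frame, using a Delay to flip the Timer direction flag about every two seconds.
; WasHit plays a collapse sound, notifies the first Score actor found and rotates Arrow 90 degrees.
; A Dead flag blocks repeat hits until the rotation reverses five seconds later.
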(event EventTick
  (params (DeltaSeconds :type Float%20%28single-precision%29))
  (bind _arrow (Variables|Default|GetArrow))
  (if (Variables|Default|Gettimer)
    (Transformation|AddLocalOffset _arrow (Math|Vector|MakeVector 0.0 0.0 (* 0.5 1.0)) false false)
    (Utilities|FlowControl|Delay 2.0)
    (Variables|Default|Settimer false)
    (else
      (Transformation|AddLocalOffset _arrow (Math|Vector|MakeVector 0.0 0.0 (* 0.5 -1.0)) false false)
      (Utilities|FlowControl|Delay 2.0)
      (Variables|Default|Settimer true))))

(event EventWasHit
  (bind _outactors (Actor|GetAllActorsOfClass "/Game/Custom/Blueprints/Score.Score_C"))
  (Variables|Default|SetScoreBoard (Utilities|Array|Get(acopy) _outactors))
  (if (not (Variables|Default|GetDead))
    (Audio|PlaySound2D "/Game/Custom/Sounds/Audio/Collapse01.Collapse01")
    (Class|ScoreInterface|Score(Message) (Variables|Default|GetScoreBoard))
    (Transformation|AddLocalRotation (Variables|Default|GetArrow) "0,-90.000000, 0" false false)
    (Variables|Default|SetDead true)
    (Utilities|FlowControl|Delay 5.0)
    (Transformation|AddLocalRotation (Variables|Default|GetArrow) "0,90.000000, 0" false false)
    (Variables|Default|SetDead false)))

(fn ConstructionScript)