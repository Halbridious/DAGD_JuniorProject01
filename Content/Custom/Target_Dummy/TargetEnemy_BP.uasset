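; Target dummy enemy that walks toward the player and is destroyed when hit.
; Tick issues a single AI MoveTo toward the first player pawn, gated by a Moving flag.
; WasHit looks up the Score actor and stores it as ScoreBoard without updating it, then destroys the enemy once, guarded by a Dead flag.
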(event EventWasHit
  ;[1 1 1] If hit kills actor
  (bind _outactors (Actor|GetAllActorsOfClass "/Game/Custom/Functionality/Score.Score_C"))
  (Variables|Default|SetScoreBoard (Utilities|Array|Get(acopy) _outactors))
  (if (not (Variables|Default|GetDead))
    (Variables|Default|SetDead true)
    (Actor|DestroyActor)))

(event EventTick
  (params (DeltaSeconds :type Float%20%28single-precision%29))
  ;[1 1 1] Moves to target point
  (if (not (Variables|Default|GetMoving))
    (AI|AIMoveTo self "0, 0, 0" (Game|Player|GetPlayerPawn 0) 5.0 false
      (:then
        (Variables|Default|SetMoving true)))))

(fn ConstructionScript)