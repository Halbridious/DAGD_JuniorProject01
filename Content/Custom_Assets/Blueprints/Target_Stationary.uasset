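; Stationary shooting target that flips on a random delay at start, then resets itself after each hit.
; WasHit always notifies the Accuracy actor, but only a live target plays a collapse sound and messages the Score actor.
; A live hit rotates the Arrow component down and sets Dead until a timed delay restores it.
; Tick keeps the Cube component turned toward the player pawn.
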(event EventBeginPlay
  ;[1 1 1] Start Down
  (Utilities|FlowControl|Delay (Math|Random|RandomFloatinRange 0.0 1e+01))
  (Transformation|AddLocalRotation (Variables|Default|GetArrow) "0,90.000000, 0" false false)
  (Audio|PlaySoundatLocation "/Game/Custom_Assets/Sounds/Ambient/387484__cosmicembers__empty-gun-failure-to-fire-trigger-pull-3.387484__cosmicembers__empty-gun-failure-to-fire-trigger-pull-3" (Transformation|GetActorLocation))
  (Variables|Default|SetDead false))

(event EventTick
  (params (DeltaSeconds :type Float%20%28single-precision%29))
  ;[1 1 1] Look at player
  (Transformation|SetWorldRotation (Variables|Default|GetCube) (Math|Rotator|FindLookatRotation (Transformation|GetWorldLocation (Variables|Default|GetCube)) (Transformation|GetActorLocation (Game|Player|GetPlayerPawn 0))) false false))

(event EventWasHit
  ;[1 1 1] Target was hit
  (bind _outactors (Actor|GetAllActorsOfClass "/Game/Custom_Assets/Blueprints/Score.Score_C"))
  (Variables|Default|SetScoreBoard (Utilities|Array|Get(acopy) _outactors))
  (bind _outactors_2 (Actor|GetAllActorsOfClass "/Game/Custom_Assets/Blueprints/Accuracy.Accuracy_C"))
  (Default|Score (Utilities|Array|Get(acopy) _outactors_2))
  (if (not (Variables|Default|GetDead))
    (Audio|PlaySound2D "/Game/Custom_Assets/Sounds/Audio/Collapse01.Collapse01")
    (Class|ScoreInterface|Score(Message) (Variables|Default|GetScoreBoard))
    (Transformation|AddLocalRotation (Variables|Default|GetArrow) "0,-90.000000, 0" false false)
    (Variables|Default|SetDead true)
    (Utilities|FlowControl|Delay 5.0)
    (Transformation|AddLocalRotation (Variables|Default|GetArrow) "0,90.000000, 0" false false)
    (Variables|Default|SetDead false)))

(fn ConstructionScript)