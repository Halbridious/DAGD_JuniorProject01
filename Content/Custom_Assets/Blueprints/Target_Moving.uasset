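; Moving shooting target that slides back and forth, falls when hit and resets after five seconds.
; Tick nudges the Arrow component along local Z by a fixed per-frame step, reversing via a Delay-toggled flag.
; WasHit always calls Score on the level's Accuracy actor.
; If standing, it also plays a collapse sound, messages the Score actor and rotates the Arrow until reset.
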(event EventTick
  (params (DeltaSeconds :type Float%20%28single-precision%29))
  (bind _arrow (Variables|Default|GetArrow))
  ;[1 1 1] Target move
  (if (Variables|Default|Gettimer)
    (Transformation|AddLocalOffset _arrow (Math|Vector|MakeVector 0.0 0.0 (* 0.5 1.0)) false false)
    (Utilities|FlowControl|Delay 2.0)
    (Variables|Default|Settimer false)
    (else
      (Transformation|AddLocalOffset _arrow (Math|Vector|MakeVector 0.0 0.0 (* 0.5 -1.0)) false false)
      (Utilities|FlowControl|Delay 2.0)
      (Variables|Default|Settimer true))))

(event EventWasHit
  ;[1 1 1] Target was hit
  (bind _outactors (Actor|GetAllActorsOfClass "/Game/Custom_Assets/Blueprints/Score.Score_C"))
  (Variables|Default|SetScoreBoard (Utilities|Array|Get(acopy) _outactors))
  (bind _outactors_2 (Actor|GetAllActorsOfClass "/Game/Custom_Assets/Blueprints/Accuracy.Accuracy_C"))
  (Default|Score (Utilities|Array|Get(acopy) _outactors_2))
  (if (not (Variables|Default|GetDead))
    (Audio|PlaySound2D "/Game/Custom_Assets/Sounds/Audio/Collapse01.Collapse01")
    (Class|ScoreInterface|Score(Message) (Variables|Default|GetScoreBoard))
    (Transformation|AddLocalRotation (Variables|Default|GetArrow) "0,-90.000000, 0" false false)
    (Variables|Default|SetDead true)
    (Utilities|FlowControl|Delay 5.0)
    (Transformation|AddLocalRotation (Variables|Default|GetArrow) "0,90.000000, 0" false false)
    (Variables|Default|SetDead false)))

(fn ConstructionScript)