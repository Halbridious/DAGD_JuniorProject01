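; Wave counter Blueprint that tracks a score, shows it on a text component and ends the level once it reaches a threshold.
; Tick writes the score to ScoreText every frame.
; The Score event increments the value behind a short delayed gate that ignores rapid repeat calls, then opens the Homecoming_IntroDemo level when the score reaches eleven.
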(event EventTick
  (params (DeltaSeconds :type Float%20%28single-precision%29))
  ;[1 1 1] display wave
  (Rendering|Components|TextRender|SetText (Variables|Default|GetScoreText) (Utilities|Text|ToText(Integer) (Variables|Default|GetScore_V))))

(event EventScore
  ;[1 0.01618 0] Score
  (if (Variables|Default|GetDoOnce)
    (Variables|Default|SetDoOnce false)
    (bind _output_get (Variables|Default|SetScore_V (+ (Variables|Default|GetScore_V) 1)))
    (Utilities|FlowControl|Delay 0.2)
    (Variables|Default|SetDoOnce true)
    (if (>= (Variables|Default|GetScore_V) 11)
      (Game|OpenLevel(byName) "Homecoming_IntroDemo"))))

(fn ConstructionScript)