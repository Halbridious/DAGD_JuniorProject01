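; Tazer weapon actor that can be picked up, dropped and fired.
; Interact flip-flops between snapping it to the given hand and detaching it, toggling mesh collision, grip offsets and the Holding flag.
; While held, Action line-traces forward from Shoot with debug drawing; a hit plays a spark sound at the tazer, spawns sparks at impact and calls WasHitMessage on BPI_Enemy actors.
; Physics simulation toggles are present but unwired.
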(event EventAction
  (bind _shoot (Variables|Default|GetShoot))
  (bind _returnvalue (Transformation|GetWorldTransform _shoot))
  ;[1 1 1] Fire Bullet
  (if (Variables|Default|GetHolding)
    (bind (_outhit _returnvalue_2) (Collision|LineTraceByChannel (.location _returnvalue) (+ (.location _returnvalue) (* (Math|Vector|GetForwardVector (.rotation _returnvalue)) 5e+03)) "TraceTypeQuery1" true 0 "ForDuration"))
    (if _returnvalue_2
      (Variables|Default|SetHit%20Actor (.HitActor (Collision|BreakHitResult _outhit)))
      (Audio|PlaySoundatLocation "/Game/Custom_Assets/Sounds/Audio/Fire_Sparks01_Cue.Fire_Sparks01_Cue" (Transformation|GetActorLocation) "0, 0, 0" 0.25)
      (Effects|SpawnEmitteratLocation "/Game/Custom_Assets/Particles/Particles/P_Sparks.P_Sparks" (.Location (Collision|BreakHitResult _outhit)))
      (if (Utilities|DoesObjectImplementInterface (Variables|Default|GetHit%20Actor) "/Game/Default_Assets/VirtualRealityBP/Blueprints/BPI_Enemy.BPI_Enemy_C")
        (Class|BPIEnemy|WasHit(Message) (Variables|Default|GetHit%20Actor))))))

(event EventInteract
  (params (Hand :type Scene%20Component%20Object%20Reference))
  (bind _glockbottom (Variables|Default|GetGlockBottom))
  (bind _defaultsceneroot (Variables|Default|GetDefaultSceneRoot))
  (Utilities|FlowControl|FlipFlop
    (:A
      ;[1 1 1] Pick up
      (Transformation|AttachComponentToComponent Hand "None" "SnapToTarget" "SnapToTarget" "KeepWorld" true)
      (Collision|SetCollisionEnabled _glockbottom "NoCollision")
      (Transformation|AddLocalRotation _defaultsceneroot "-45.000000,0.000000,0.000000" false false) ; Fix rotation
      (Transformation|AddLocalOffset _glockbottom "2.000000, 0, 0" false false) ; Fix Location
      (Variables|Default|SetHolding true))
    (:B
      ;[1 1 1] Drop
      (Transformation|DetachFromActor "KeepWorld" "KeepWorld" "KeepWorld")
      (Collision|SetCollisionEnabled _glockbottom "QueryAndPhysics")
      (Transformation|AddLocalRotation _defaultsceneroot "45.000000,0.000000,0.000000" false false) ; Fix rotation
      (Transformation|AddLocalOffset _glockbottom "-2.000000, 0, 0" false false) ; Fix Location
      (Variables|Default|SetHolding false))))

(fn ConstructionScript)