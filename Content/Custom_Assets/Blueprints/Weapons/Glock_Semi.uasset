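; Semi-automatic Glock pistol that can be picked up and dropped through Interact, toggling attachment to the hand, collision and crosshair visibility.
; While held, Action fires a hitscan trace from the Shoot component, spawns an impact effect and notifies hit actors implementing BPI_Enemy.
; Each shot plays a gunshot, fakes slide recoil with delayed mesh offsets, ejects a bullet actor and reports to the Accuracy actor.
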(event EventAction
  (bind _shoot (Variables|Default|GetShoot))
  (bind _returnvalue (Transformation|GetWorldTransform _shoot))
  ;[1 1 1] Fire Bullet
  (if (Variables|Default|GetHolding)
    (bind _outactors (Actor|GetAllActorsOfClass "/Game/Custom_Assets/Blueprints/Accuracy.Accuracy_C"))
    (Class|ScoreInterface|BulletsFired(Message) (Utilities|Array|Get(acopy) _outactors))
    (bind _outhit (Collision|LineTraceByChannel (.location _returnvalue) (+ (.location _returnvalue) (* (Math|Vector|GetForwardVector (.rotation _returnvalue)) 2e+04)) "TraceTypeQuery1" true 0 "None"))
    (Variables|Default|SetHitActor (.HitActor (Collision|BreakHitResult _outhit)))
    (Audio|PlaySoundatLocation "/Game/Custom_Assets/Sounds/GunShot.GunShot" (Transformation|GetActorLocation) "0, 0, 0" 0.25)
    (CallFunction|GunFunction01)
    (Utilities|FlowControl|Delay 0.01)
    (CallFunction|BulletEjection)
    (Utilities|FlowControl|Delay 0.01)
    (CallFunction|GunFunction02)
    (Effects|SpawnEmitteratLocation "/Game/Custom_Assets/Particles/Particles/BulletSplash.BulletSplash" (.Location (Collision|BreakHitResult _outhit)))
    (bind _outactors_2 (Actor|GetAllActorsOfClass "/Game/Custom_Assets/Blueprints/Accuracy.Accuracy_C"))
    (Default|BulletsFired (Utilities|Array|Get(acopy) _outactors_2))
    (if (Utilities|DoesObjectImplementInterface (Variables|Default|GetHitActor) "/Game/Default_Assets/VirtualRealityBP/Blueprints/BPI_Enemy.BPI_Enemy_C")
      (Class|BPIEnemy|WasHit(Message) (Variables|Default|GetHitActor)))))

(event EventInteract
  (params (Hand :type Scene%20Component%20Object%20Reference))
  (bind _glockbottom (Variables|Default|GetGlockBottom))
  (bind _defaultsceneroot (Variables|Default|GetDefaultSceneRoot))
  (Utilities|FlowControl|FlipFlop
    (:A
      ;[1 1 1] Pick up
      (Transformation|AttachComponentToComponent Hand "None" "SnapToTarget" "SnapToTarget" "KeepRelative" true)
      (Collision|SetCollisionEnabled _glockbottom "NoCollision")
      (Transformation|AddLocalRotation _defaultsceneroot "-45.000000,0.000000,0.000000" false false) ; Fix rotation
      (Transformation|AddLocalOffset _glockbottom "2.000000, 0, 0" false false) ; Fix Location
      (Variables|Default|SetHolding true)
      (Rendering|ToggleVisibility (Variables|Default|GetCrossHairs) false))
    (:B
      ;[1 1 1] Drop
      (Transformation|DetachFromActor "KeepWorld" "KeepWorld" "KeepWorld")
      (Collision|SetCollisionEnabled _glockbottom "QueryAndPhysics")
      (Transformation|AddLocalRotation _defaultsceneroot "45.000000,0.000000,0.000000" false false) ; Fix rotation
      (Transformation|AddLocalOffset _glockbottom "-2.000000, 0, 0" false false) ; Fix Location
      (Variables|Default|SetHolding false)
      (Rendering|ToggleVisibility (Variables|Default|GetCrossHairs) false))))

(fn ConstructionScript
  (|CallParentFunction))

(fn GunFunction01
  (Transformation|AddLocalOffset (Variables|Default|GetGlockTop) (Variables|Default|GetStartFireTransform) false false))

(fn GunFunction02
  (Transformation|AddLocalOffset (Variables|Default|GetGlockTop) "1.000000, 0, 0" false false))

(fn BulletEjection
  (Game|SpawnActorfromClass "/Game/Default_Assets/VirtualRealityBP/Blueprints/BulletEject_BP.BulletEject_BP_C" (Math|Transform|MakeTransform (.location (Transformation|GetWorldTransform (Variables|Default|GetEjection))) "0, 0, 0" "1,1,1") "Undefined" 0 0))