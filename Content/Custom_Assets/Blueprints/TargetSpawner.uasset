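; Target spawner that periodically spawns enemy or friendly AI targets at its Arrow component's transform.
; After an initial delay on BeginPlay, a looping timer triggers a spawn attempt.
; Two random rolls decide whether a target appears and then whether it is TargetEnemy_BP or TargetFriendly_BP.
; Leftover logic that calls ScoreMessage on the Wave actor and sets NewRound is disconnected and never runs.
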(event Custom|SpawnTarget
  (bind _arrow (Variables|Default|GetArrow))
  (bind _returnvalue (Transformation|GetWorldLocation _arrow))
  (bind _returnvalue_2 (Transformation|GetWorldRotation _arrow))
  ;[1 1 1] Random spawn
  (if (<= (Math|Random|RandomFloatinRange -7.0 5.0) 0.0)
    ;[1 1 1] Spawns target every few seconds
    (if (<= (Math|Random|RandomFloatinRange -5.0 5.0) 0.0)
      (AI|SpawnAIFromClass "/Game/Custom_Assets/Blueprints/TargetEnemy_BP.TargetEnemy_BP_C" 0 _returnvalue _returnvalue_2 false)
      (else
        (AI|SpawnAIFromClass "/Game/Custom_Assets/Blueprints/TargetFriendly_BP.TargetFriendly_BP_C" 0 _returnvalue _returnvalue_2 false)))))

(event Custom|SpawnTargets
  ;[1 1 1] Starts new round
  (CallFunction|SpawnTarget))

(event EventBeginPlay
  (Utilities|FlowControl|Delay 5.0)
  (Utilities|Time|SetTimerbyEvent (delegate Custom|SpawnTargets) 3.0 true))

(fn ConstructionScript)