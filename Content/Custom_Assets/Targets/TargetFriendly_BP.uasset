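; Friendly target pawn that moves around the level and triggers the game-finished message when hit.
; On Tick it issues a single AI move to a random reachable point around a stored origin, latched by a Moving flag that is never cleared.
; The first hit plays a sound, marks it dead, toggles mesh visibility without destroying the actor, and notifies the first MotionControllerPawn found.
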(event EventWasHit
  ;[1 1 1] If hit kills actor
  (if (not (Variables|Default|GetDead))
    (Audio|PlaySound2D 0)
    (Variables|Default|SetDead true)
    (Rendering|ToggleVisibility (Variables|Character|GetMesh) false)
    (bind _outactors (Actor|GetAllActorsOfClass "/Game/Default_Assets/VirtualRealityBP/Blueprints/MotionControllerPawn.MotionControllerPawn_C"))
    (Class|PostGameInterface|GameFinished(Message) (Utilities|Array|Get(acopy) _outactors))))

(event EventTick
  (params (DeltaSeconds :type Float%20%28single-precision%29))
  ;[1 1 1] Moves to target point
  (if (not (Variables|Default|GetMoving))
    (AI|AIMoveTo self (.RandomLocation (AI|Navigation|GetRandomReachablePointinRadius (Variables|Default|GetNewVar_0) 1e+04)) 0 5.0 false
      (:then
        (Variables|Default|SetMoving true)))))

(fn ConstructionScript)