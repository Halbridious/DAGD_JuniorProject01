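; Procedural building generator actor that assembles modular static meshes in its construction script from floor count, width, length and an optional door position.
; Each floor gets a front wall row, side walls and corner edges, spaced by the wall mesh bounds, with the door replacing one ground-floor panel.
; Walls and door get dynamic material instances tinted by BrickColor.
; Side-wall loops ignore their index, so pieces overlap; edge-cap code is unconnected.
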(event EventBeginPlay)

(event Collision|EventActorBeginOverlap
  (params (OtherActor :type Actor%20Object%20Reference)))

(event EventTick
  (params (DeltaSeconds :type Float%20%28single-precision%29)))

(fn ConstructionScript
  (bind _meshwall (Variables|Default|GetMeshWall))
  (bind _widthofbuilding (Variables|Default|GetWidthOfBuilding))
  (bind _meshwall_2 (Variables|Default|GetMeshWall))
  (bind _meshwall_3 (Variables|Default|GetMeshWall))
  (bind _returnvalue (- _widthofbuilding 1))
  (bind _returnvalue_2 (StaticMesh|GetBounds _meshwall_3))
  (bind _returnvalue_3 (StaticMesh|GetBounds _meshwall_2))
  (bind _returnvalue_4 (StaticMesh|GetBounds _meshwall))
  (bind _boxextent (Math|BoxSphereBounds|BreakBoxSphereBounds _returnvalue_3))
  (bind _boxextent_2 (Math|BoxSphereBounds|BreakBoxSphereBounds _returnvalue_2))
  (bind _boxextent_3 (Math|BoxSphereBounds|BreakBoxSphereBounds _returnvalue_4))
  (bind (_x _y) (Math|Vector|BreakVector _boxextent_2))
  (bind (_x_2 _y_2) (Math|Vector|BreakVector _boxextent))
  (bind _x_3 (Math|Vector|BreakVector _boxextent_3))
  (bind _returnvalue_5 (* _x_3 -1.0))
  (for _index (range 0 (- (Variables|Default|GetNumbeOfFloors) 1))
    (bind _returnvalue_6 (AddComponent|AddStaticMeshComponent false (Math|Transform|MakeTransform (Math|Vector|MakeVector (- (* _x -1.0) 5.2) -4.8 (* _index (* _y 2.0))) "0, 0,90.000000")))
    (Components|StaticMesh|SetStaticMesh _returnvalue_6 (Variables|Default|GetMeshEdge))
    (Utilities|FlowControl|Sequence
      (:then_0
        (for _index_2 (range 0 _returnvalue)
          (Utilities|FlowControl|Sequence
            (:then_0
              (if (Variables|Default|GetHasDoor)
                (if (== _index 0)
                  (if (== _index_2 (- (Variables|Default|GetDoorLocation) 1))
                    (bind _returnvalue_7 (AddComponent|AddStaticMeshComponent false (Math|Transform|MakeTransform (Math|Vector|MakeVector (* _index_2 (* (.X (Math|Vector|BreakVector (.BoxExtent (Math|BoxSphereBounds|BreakBoxSphereBounds (StaticMesh|GetBounds (Variables|Default|GetMeshWall)))))) 2.0)) 0.0 (* _index (* _y 2.0))) "0, 0,90.000000")))
                    (Components|StaticMesh|SetStaticMesh _returnvalue_7 (Variables|Default|GetMeshDoor))
                    (bind _returnvalue_8 (Rendering|Material|CreateDynamicMaterialInstance _returnvalue_7 0 "/Game/Custom_Assets/BuildingGenerator/Models/DoorMat.DoorMat" :!class /Script/Engine.PrimitiveComponent))
                    (Rendering|Material|SetVectorParameterValue _returnvalue_8 "BrickColor" (Variables|Default|GetBrickColor) :!class /Script/Engine.MaterialInstanceDynamic)
                    (else
                      (bind _returnvalue_9 (AddComponent|AddStaticMeshComponent false (Math|Transform|MakeTransform (Math|Vector|MakeVector (* _index_2 (* (.X (Math|Vector|BreakVector (.BoxExtent (Math|BoxSphereBounds|BreakBoxSphereBounds (StaticMesh|GetBounds (Variables|Default|GetMeshWall)))))) 2.0)) 0.0 (* _index (* _y 2.0))) "0, 0,90.000000") :!label _label))
                      (Components|StaticMesh|SetStaticMesh _returnvalue_9 (Variables|Default|GetMeshWall))
                      (bind _returnvalue_10 (Rendering|Material|CreateDynamicMaterialInstance _returnvalue_9 0 "/Game/Custom_Assets/BuildingGenerator/Models/PanelMat.PanelMat" :!class /Script/Engine.PrimitiveComponent))
                      (Rendering|Material|SetVectorParameterValue _returnvalue_10 "BrickColor" (Variables|Default|GetBrickColor) :!class /Script/Engine.MaterialInstanceDynamic)))
                  (else
                    (goto _label)))
                (else
                  (goto _label))))
            (:then_1
              (if (== _index_2 _returnvalue)
                (Utilities|FlowControl|Sequence
                  (:then_0
                    (for _index_3 (range 0 (- (Variables|Default|GetLenghtOfBuilding) 1))
                      (bind _returnvalue_11 (AddComponent|AddStaticMeshComponent false (Math|Transform|MakeTransform (Math|Vector|MakeVector (+ (* _index_2 (* (.X (Math|Vector|BreakVector (.BoxExtent (Math|BoxSphereBounds|BreakBoxSphereBounds (StaticMesh|GetBounds (Variables|Default|GetMeshWall)))))) 2.0)) _y_2) (* _x_2 -1.0) (* _index (* _y 2.0))) "0.000000,-90.000000,90.000000")))
                      (Components|StaticMesh|SetStaticMesh _returnvalue_11 (Variables|Default|GetMeshWall))
                      (bind _returnvalue_12 (Rendering|Material|CreateDynamicMaterialInstance _returnvalue_11 0 "/Game/Custom_Assets/BuildingGenerator/Models/PanelSideMat.PanelSideMat" :!class /Script/Engine.PrimitiveComponent))
                      (Rendering|Material|SetVectorParameterValue _returnvalue_12 "BrickColor" (Variables|Default|GetBrickColor) :!class /Script/Engine.MaterialInstanceDynamic)))
                  (:then_1
                    (bind _returnvalue_13 (AddComponent|AddStaticMeshComponent false (Math|Transform|MakeTransform (Math|Vector|MakeVector (+ (+ (* _index_2 (* (.X (Math|Vector|BreakVector (.BoxExtent (Math|BoxSphereBounds|BreakBoxSphereBounds (StaticMesh|GetBounds (Variables|Default|GetMeshWall)))))) 2.0)) _x_2) 5.2) -4.8 (* _index (* _y 2.0))) "0, 0,90.000000" (Math|Vector|MakeVector (* 0.0 -1.0) 0.0 0.0))))
                    (Components|StaticMesh|SetStaticMesh _returnvalue_13 (Variables|Default|GetMeshEdge)))))))))
      (:then_1
        (for _index_4 (range 0 (- (Variables|Default|GetLenghtOfBuilding) 1))
          (bind _returnvalue_14 (AddComponent|AddStaticMeshComponent false (Math|Transform|MakeTransform (Math|Vector|MakeVector _returnvalue_5 _returnvalue_5 (* _index (* _y 2.0))) "0.000000,90.000000,90.000000")))
          (Components|StaticMesh|SetStaticMesh _returnvalue_14 (Variables|Default|GetMeshWall))
          (bind _returnvalue_15 (Rendering|Material|CreateDynamicMaterialInstance _returnvalue_14 0 "/Game/Custom_Assets/BuildingGenerator/Models/PanelSideMat.PanelSideMat" :!class /Script/Engine.PrimitiveComponent))
          (Rendering|Material|SetVectorParameterValue _returnvalue_15 "BrickColor" (Variables|Default|GetBrickColor) :!class /Script/Engine.MaterialInstanceDynamic))))))